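; BP_Player is a player pawn that handles movement input and switching between camera views.
; MoveForward and MoveRight axes feed movement input along fixed world Y and X, independent of camera or pawn facing.
; The ChangeCamera action checks which key was pressed: 1 sets the player controller's view target to OverworldCamera, 2 returns it to the controlled pawn.
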(event `InputAxis|MoveForward`
  (params (AxisValue :type "Float (single-precision)"))
  (`self.AddMovementInput` (0.0 1.0 0.0) AxisValue))

(event `InputAxis|MoveRight`
  (params (AxisValue :type "Float (single-precision)"))
  (`self.AddMovementInput` (1.0 0.0 0.0) AxisValue))

(event `InputAction|ChangeCamera`
  (params (Key :type "Key Structure" :default "AnyKey"))
  (bind _returnvalue (`GameplayStatics.GetPlayerController` 0))
  (:`Pressed`
    (if (== Key "One")
      (`PlayerController.SetViewTargetWithBlend` _returnvalue (`self.OverworldCamera`) 0.0 "VTBlend_Linear" 0.0 false)
      (elif (== Key "Two")
        (`PlayerController.SetViewTargetWithBlend` _returnvalue (`Controller.K2_GetPawn` _returnvalue) 0.0 "VTBlend_Linear" 0.0 false)))))

(fn `UserConstructionScript`)