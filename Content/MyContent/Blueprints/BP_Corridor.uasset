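; BP_Corridor is a corridor piece whose floor is sized from a CorridorLength input.
; The construction script scales the Floor along X by that length with fixed width and thickness, then shifts it forward by half the length so it extends from the root.
; The Horizontal flag picks whether the floor sits at a positive or negative Y offset.
; The event graph has no active logic.
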(fn `UserConstructionScript`
  (bind _floor (`self.Floor`))
  (bind _returnvalue (`KismetMathLibrary.Conv_IntToDouble` (`self.CorridorLength`)))
  (bind _returnvalue_2 (/ (* _returnvalue 100.0) 2.0))
  ;[1 1 1] Scale the corridor length based on input length. The location of the floor must act as if the default scene root is 0,0,0 so set relative location of the floor based on this input length
  (`SceneComponent.SetRelativeScale3D` (`self.Floor`) (`KismetMathLibrary.MakeVector` _returnvalue 3.0 0.1))
  (if (`self.Horizontal?`)
    (bind _output_get (set `self.yPosition` 300.0))
    (`SceneComponent.K2_SetRelativeLocation` _floor (`KismetMathLibrary.MakeVector` _returnvalue_2 _output_get 0.0) false false)
    (else
      (bind _output_get_2 (set `self.yPosition` -300.0))
      (`SceneComponent.K2_SetRelativeLocation` _floor (`KismetMathLibrary.MakeVector` _returnvalue_2 _output_get_2 0.0) false false))))