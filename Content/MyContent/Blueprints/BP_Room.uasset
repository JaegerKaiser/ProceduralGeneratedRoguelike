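; BP_Room is a room actor whose floor is sized in the editor from the FloorX and FloorY inputs.
; The construction script scales the thin Floor component by those lengths, then offsets it by half its size in 100-unit steps, keeping the scene root at a corner of the floor.
; The event graph holds only disabled default events, so it adds no runtime logic.
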(fn `UserConstructionScript`
  (bind _returnvalue (`KismetMathLibrary.Conv_IntToDouble` (`self.FloorX`)))
  (bind _returnvalue_2 (`KismetMathLibrary.Conv_IntToDouble` (`self.FloorY`)))
  ;[1 1 1] Scale the room based on input lengths. The location of the floor must act as if the default scene root is 0,0,0 so set relative location of the floor based on these input lengths
  (`SceneComponent.SetRelativeScale3D` (`self.Floor`) (`KismetMathLibrary.MakeVector` _returnvalue _returnvalue_2 0.1))
  (`SceneComponent.K2_SetRelativeLocation` (`self.Floor`) (`KismetMathLibrary.MakeVector` (/ (* _returnvalue 100.0) 2.0) (/ (* _returnvalue_2 100.0) 2.0) 0.0) false false))